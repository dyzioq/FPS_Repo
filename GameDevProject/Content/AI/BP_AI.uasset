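; BP_AI is the enemy character in a survival game, taking damage and making melee attacks.
; Damage lowers Health; at zero it ragdolls, stops moving, reports the kill to BP_SurviveGameMod and is destroyed after a delay, with IsDead blocking repeat deaths.
; Attack plays a montage whose notify fires a short forward sphere trace for pawns, ignoring actors tagged Bot, and damages the hit actor.
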(event EventAttack
  (bind _returnvalue (Transformation|GetActorLocation))
  ;[1 1 1] When Enemy attack play animation and apply damage
  (if (not (Variables|Default|GetisDead))
    (Animation|Montage|PlayMontage (Variables|Character|GetMesh) "/Game/Characters/Mannequins/Animations/Attack_Montage.Attack_Montage"
      (:OnNotifyBegin
        (bind _outactors (Actor|GetAllActorswithTag "Bot"))
        (bind (_outhit _returnvalue_2) (Collision|SphereTraceForObjects _returnvalue (+ _returnvalue (* (Math|Vector|GetForwardVector (Transformation|GetActorRotation)) 1.7e+02)) 3e+01 (Utilities|Array|MakeArray "ObjectTypeQuery3") false _outactors "None"))
        (if _returnvalue_2
          (Game|Damage|ApplyDamage (.HitActor (Collision|BreakHitResult _outhit)) 1e+01 0 0))))))

(event Game|Damage|EventAnyDamage
  (params (Damage :type Float%20%28single-precision%29) (DamageType :type Damage%20Type%20Object%20Reference) (InstigatedBy :type Controller%20Object%20Reference) (DamageCauser :type Actor%20Object%20Reference))
  ;[1 1 1] Apply damage towards Enemy, check if Enemy is dead
  ;[1 1 1] check if is dead to avoid killing the same enemy multiple times
  (if (not (Variables|Default|GetisDead))
    (Variables|Default|Sethealth (- (Variables|Default|Gethealth) Damage))
    (if (<= (Variables|Default|Gethealth) 0.0)
      (Variables|Default|SetisDead true)
      (Physics|SetSimulatePhysics (Variables|Character|GetMesh) true)
      (Pawn|Components|CharacterMovement|DisableMovement (Variables|Character|GetCharacterMovement))
      (bind _asbp_survive_game_mod (Utilities|Casting|CastToBP_SurviveGameMod (Game|GetGameMode)))
      (Default|EnemyKilled _asbp_survive_game_mod)
      (Utilities|FlowControl|Delay 3.0)
      (Actor|DestroyActor))))

(fn ConstructionScript)